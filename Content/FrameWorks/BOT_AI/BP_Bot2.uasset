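; AI-controlled rifle bot for Team Deathmatch, tagged with its team on construction.
; FireBullet line-traces from the rifle to the AI controller's focus actor, applying point damage, gunshot audio and an impact effect.
; Non-lethal hits are reported to AI damage sensing.
; At zero health it unpossesses, ragdolls the mesh with a death animation, updates the game state's team score and expires shortly after.
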(event Custom|Fire%20Bullet
  (bind _self self)
  (bind _returnvalue (AI|GetAIController _self))
  (bind _returnvalue_2 (Class|AIController|GetFocusActor _returnvalue))
  ;[1 1 1] shooting mechanic
  (Utilities|IsValid _returnvalue_2
    (:Is%20Valid
      (bind (_outhit _returnvalue_3) (Collision|LineTraceByChannel (Transformation|GetWorldLocation (Variables|Default|GetRifle_AR)) (Transformation|GetActorLocation _returnvalue_2) "TraceTypeQuery1" false 0 "ForDuration"))
      (Game|Damage|ApplyPointDamage (.HitActor (Collision|BreakHitResult _outhit)) 1e+01 (.ImpactNormal (Collision|BreakHitResult _outhit)) _outhit 0 self)
      (Audio|PlaySoundatLocation "/Game/ThirdPerson/Sounds/AR_Shoot_Cue.AR_Shoot_Cue" (Transformation|GetActorLocation) "0, 0, 0" 1.0 1.0 0.0 0 0 0 0)
      (if _returnvalue_3
        (Niagara|SpawnSystematLocation 0 (.Location (Collision|BreakHitResult _outhit)) (Math|Rotator|MakeRotfromX (.ImpactNormal (Collision|BreakHitResult _outhit))))))))

(event Custom|Enemy%20Death
  (bind _mesh (Variables|Character|GetMesh))
  (Pawn|UnPossess (AI|GetAIController self))
  (Collision|SetCollisionEnabled _mesh "PhysicsOnly")
  (Physics|SetSimulatePhysics _mesh true)
  (Collision|SetCollisionEnabled (Variables|Collision|GetCapsuleComponent) "NoCollision")
  (Components|Animation|PlayAnimation (Variables|Character|GetMesh) "/Game/AnimStarterPack/Death_2.Death_2" false)
  (Actor|SetLifeSpan 2.0))

(event EventBeginPlay)

(event Collision|EventActorBeginOverlap
  (params (OtherActor :type Actor%20Object%20Reference)))

(event Game|Damage|EventAnyDamage
  (params (Damage :type Float%20%28single-precision%29) (DamageType :type Damage%20Type%20Object%20Reference) (InstigatedBy :type Controller%20Object%20Reference) (DamageCauser :type Actor%20Object%20Reference))
  (bind _output_get (Variables|Default|SetCurrentHeatlh (- (Variables|Default|GetCurrentHeatlh) Damage)))
  (if (<= _output_get 0.0)
    (CallFunction|EnemyDeath)
    (bind _asgs_team_death_match (Utilities|Casting|CastToGS_TeamDeathMatch (Game|GetGameState)))
    (Default|IncreasePointby1forTeams _asgs_team_death_match (== (Variables|Default|GetTeams) 10))
    (else
      (Class|AISenseDamage|ReportDamageEvent self DamageCauser Damage (Transformation|GetActorLocation) "0, 0, 0" "None"))))

(fn ConstructionScript
  (GameplayTags|AddGameplayTag (Variables|Default|GetActorTypeContainer) (Variables|Default|GetTeamTag) :!class /Script/GameplayTags.BlueprintGameplayTagLibrary))