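; Team deathmatch game mode that balances joining players into two three-player teams and runs the pre-match countdown.
; PostLogin alternates via FlipFlop, storing controllers per team and tagging PlayerStates; Team 1 overflows into Team 2, and a full Team 2 opens MainMenu.
; A one-shot pre-match timer starts the looping get-ready countdown if its counter expires or both teams are full.
; When that countdown ends, StartMatch flags the match as started.
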(event Custom|PreMatch%20Timer%20Event
  ;[1 1 1] BeginPlay
  (bind _result (Math|Float|DecrementFloat (Variables|Default|GetTimerCounter))
    (:%20%20
      (if (<= _result 0.0)
        (Utilities|Time|ClearandInvalidateTimerbyHandle (Variables|Default|GetPreMatchTime) :!label _label)
        (bind _returnvalue (Utilities|Time|SetTimerbyEvent (delegate Custom|GetReadyTimerEvent) 1.0 true))
        (Variables|Default|SetGetReadyTimer _returnvalue)
        (else
          (bind _returnvalue_2 (CallFunction|GetTotalControllers))
          (if (== _returnvalue_2 6)
            (goto _label)))))))

(event Custom|GetReadyTimerEvent
  ;[1 1 1] BeginPlay
  (bind _result (Math|Float|DecrementFloat (Variables|Default|GetGetReadyTimerCD))
    (:%20%20
      (Development|PrintString (Utilities|String|ToString(Float) _result))
      (if (<= _result 0.0)
        (Utilities|Time|ClearandInvalidateTimerbyHandle (Variables|Default|GetGetReadyTimer))
        (CallFunction|StartMatch)))))

(event Custom|Start%20Match
  (Variables|Default|SetMatchStart true)
  (Utilities|FlowControl|Sequence))

(event EventPostLogin
  (params (NewPlayer :type Player%20Controller%20Object%20Reference))
  ;[1 1 1] Team Balancing
  (bind _asbp_tdmplayer_controller (Utilities|Casting|CastToBP_TDMPlayerController NewPlayer))
  (Utilities|FlowControl|FlipFlop
    (:A
      (if (< (Utilities|Array|Length (Variables|Default|GetTeam1Controller)) 3)
        (Utilities|Array|Add (Variables|Default|GetTeam1Controller) _asbp_tdmplayer_controller)
        (bind _asbp_player_state (Utilities|Casting|CastToBP_PlayerState (Variables|/Script/Engine.Controller|GetPlayerState _asbp_tdmplayer_controller)))
        (Class|BPITeamInteraction|SetTeam(Message) _asbp_player_state "NewEnumerator0")
        (else
          (if (< (Utilities|Array|Length (Variables|Default|GetTeam2Controller)) 3) :!label _label
            (Utilities|Array|Add (Variables|Default|GetTeam2Controller) _asbp_tdmplayer_controller)
            (bind _asbp_player_state_2 (Utilities|Casting|CastToBP_PlayerState (Variables|/Script/Engine.Controller|GetPlayerState _asbp_tdmplayer_controller)))
            (Class|BPITeamInteraction|SetTeam(Message) _asbp_player_state_2 "NewEnumerator1")
            (else
              (Game|OpenLevel(byName) "MainMenu"))))))
    (:B
      (goto _label))))

(event EventBeginPlay
  ;[1 1 1] BeginPlay
  (bind _returnvalue (Utilities|Time|SetTimerbyEvent (delegate Custom|PreMatch%20Timer%20Event) 1.0))
  (Variables|Default|SetPreMatchTime _returnvalue))

(fn ConstructionScript)

(fn GetTotalControllers
  (return (+ (Utilities|Array|Length (Variables|Default|GetTeam1Controller)) (Utilities|Array|Length (Variables|Default|GetTeam2Controller)))))