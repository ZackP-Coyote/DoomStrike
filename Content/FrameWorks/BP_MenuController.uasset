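; Player controller for the menu and multiplayer lobby, giving the local player a cursor and UI-only input.
; Initial setup loads the saved player profile, creating the save slot if missing, and passes it to ServerUpdateLobby, which has BP_Menu_GM update the lobby.
; Events create or show the lobby widget and refresh its player names from supplied profiles.
; Ending a client session destroys it, then opens MainMenu.
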(event Custom|End%20Client%20Session
  (|DestroySession self
    (:then
      (Game|OpenLevel(byName) "MainMenu"))))

(event Custom|Create%20Lobby%20Menu
  (CallFunction|UIShowLobbyMenu))

(event Custom|Initial%20Setup
  (CallFunction|LoadSavedProfile)
  (CallFunction|ServerUpdateLobby (Variables|Default|GetPlayer%20Profile%20Info)))

(event Custom|Update%20Player%20Names
  (params (PlayerProfiles :type Array%20of%20S%20Player%20Profile%20Structures))
  (bind _wb_lobbymenu (Variables|Default|GetWB_LobbyMenu))
  (Utilities|IsValid _wb_lobbymenu
    (:Is%20Valid
      (Default|ClearPlayerNames _wb_lobbymenu)
      (Default|UpdatePlayerNames _wb_lobbymenu PlayerProfiles))))

(event Custom|Server%20Update%20Lobby
  (params (Player%20Profiles :type S%20Player%20Profile%20Structure))
  (Variables|Default|SetPlayer%20Profile%20Info Player%20Profiles)
  (bind _asbp_menu_gm (Utilities|Casting|CastToBP_Menu_GM (Game|GetGameMode)))
  (Default|UpdateLobby _asbp_menu_gm false))

(event EventBeginPlay
  (if (Pawn|IsLocalController)
    (Variables|Default|SetbShowMouseCursor true)
    (Input|SetInputModeUIOnly self 0 "DoNotLock" false)))

(event EventTick
  (params (DeltaSeconds :type Float%20%28single-precision%29)))

(fn ConstructionScript)

(fn UIShowLobbyMenu
  (Utilities|IsValid (Variables|Default|GetWB_LobbyMenu)
    (:Is%20Valid
      _)
    (:Is%20Not%20Valid
      (bind _returnvalue (UserInterface|CreateWidget "/Game/MainMenu/WB_LobbyMenu.WB_LobbyMenu_C" self))
      (Variables|Default|SetWB_LobbyMenu _returnvalue)))
  (UserInterface|Viewport|AddtoViewport (Variables|Default|GetWB_LobbyMenu) 0)
  (return))

(fn LoadSavedProfile
  (bind _returnvalue (SaveGame|DoesSaveGameExist (LocalVariables|GetLcl_SlotName)))
  (if _returnvalue
    _
    (else
      (bind _returnvalue_2 (SaveGame|CreateSaveGameObject "/Game/SavedData/SG_PlayerProfile.SG_PlayerProfile_C"))
      (SaveGame|SaveGametoSlot _returnvalue_2 (LocalVariables|GetLcl_SlotName))))
  (bind _returnvalue_3 (SaveGame|LoadGamefromSlot (LocalVariables|GetLcl_SlotName)))
  (bind _assg_player_profile (Utilities|Casting|CastToSG_PlayerProfile _returnvalue_3))
  (Variables|Default|SetPlayer%20Profile%20Info (Variables|/Game/SavedData/SG_PlayerProfile.SG_PlayerProfile_C|GetPlayer%20Profile _assg_player_profile))
  (return))