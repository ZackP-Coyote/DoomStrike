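; Game mode for the menu that tracks connected players in the lobby and shares their profiles with each other.
; In the Lobby Level, each new BP_MenuController is added to the player list and told to create its lobby menu and run initial setup.
; UpdateLobby rebuilds the profile list from all controllers and pushes it to each one.
; Logout removes the controller and triggers that refresh.
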(event Custom|Update%20Lobby
  (params (Player%20Names :type Boolean))
  (if Player%20Names
    (Utilities|Array|Clear (Variables|Default|GetAll%20Player%20Profiles))
    (for _array_element (Variables|Default|GetAll%20Connected%20Players)
      (Utilities|Array|Add (Variables|Default|GetAll%20Player%20Profiles) (Variables|/Game/FrameWorks/BP_MenuController.BP_MenuController_C|GetPlayer%20Profile%20Info _array_element)))
    (for _array_element_2 (Variables|Default|GetAll%20Connected%20Players)
      (if Player%20Names
        (Default|UpdatePlayerNames _array_element_2 (Variables|Default|GetAll%20Player%20Profiles))))))

(event EventHandleStartingNewPlayer
  (params (NewPlayer :type Player%20Controller%20Object%20Reference))
  (bind _returnvalue (Game|GetCurrentLevelName true))
  (switch string _returnvalue
    (:LobbyLevel
      (bind _asbp_menu_controller (Utilities|Casting|CastToBP_MenuController NewPlayer))
      (Utilities|Array|Add (Variables|Default|GetAll%20Connected%20Players) _asbp_menu_controller)
      (Default|CreateLobbyMenu _asbp_menu_controller)
      (Default|InitialSetup _asbp_menu_controller))))

(event EventOnLogout
  (params (ExitingController :type Controller%20Object%20Reference))
  (Utilities|Casting|CastToBP_MenuController ExitingController)
  (Utilities|Array|RemoveItem (Variables|Default|GetAll%20Connected%20Players) 0)
  (CallFunction|UpdateLobby true))

(fn ConstructionScript)