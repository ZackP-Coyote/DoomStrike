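; BP_AI_Character is an AI character that wanders, chases the player and can die.
; From BeginPlay it moves to random reachable points nearby, pausing and repeating only after each successful move.
; PawnSensing sighting of a BP_ThirdPersonCharacter issues an AI MoveTo toward it, with no explicit return to wandering.
; Damage reduces health; at zero or below, the mesh ragdolls and movement mode becomes None.
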(event OnSeePawn(PawnSensing)
  (params (Pawn :type Pawn%20Object%20Reference))
  ;[1 1 1] Chase Target
  (Utilities|Casting|CastToBP_ThirdPersonCharacter Pawn)
  (CallFunction|ChaseTarget Pawn))

(event Custom|Search%20Around
  ;[1 1 1] Search Around
  (AI|AIMoveTo self (.RandomLocation (AI|Navigation|GetRandomReachablePointinRadius (Transformation|GetActorLocation) 2e+03 0 0)) 0 3e+02 false
    (:OnSuccess
      (Utilities|FlowControl|Delay 1.0)
      (CallFunction|SearchAround))))

(event Custom|Chase%20Target
  (params (TargetActor :type Actor%20Object%20Reference))
  ;[1 1 1] Chase Target
  (AI|AIMoveTo self "0, 0, 0" TargetActor 5.0 false))

(event EventBeginPlay
  (CallFunction|SearchAround))

(event Game|Damage|EventAnyDamage
  (params (Damage :type Float%20%28single-precision%29) (DamageType :type Damage%20Type%20Object%20Reference) (InstigatedBy :type Controller%20Object%20Reference) (DamageCauser :type Actor%20Object%20Reference))
  ;[1 1 1] Health
  (Variables|Default|SetHealth (- (Variables|Default|GetHealth) Damage))
  (if (<= (Variables|Default|GetHealth) 0.0)
    (Physics|SetSimulatePhysics (Variables|Character|GetMesh) true)
    (Pawn|Components|CharacterMovement|SetMovementMode (Variables|Character|GetCharacterMovement) "MOVE_None" 0)))

(fn ConstructionScript)